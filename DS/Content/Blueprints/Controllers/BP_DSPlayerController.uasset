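; BP_DSPlayerController is a player controller that switches control between the Pawns in the level when Tab is pressed.
; BeginPlay caches every Pawn actor in the Players array once, without later refresh.
; Each Tab press passes NextPlayerIndex to PossessPlayer, which validates it, unpossesses and possesses that Pawn, then the index advances with wraparound.
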(event `self.ReceiveBeginPlay`
  (bind _outactors (`GameplayStatics.GetAllActorsOfClass` "/Script/Engine.Pawn"))
  (set `self.Players` _outactors))

(event `Key|Tab`
  (params (Key :type "Key Structure"))
  (:`Pressed`
    (`self.PossessPlayer` (`self.NextPlayerIndex`))
    (set `self.NextPlayerIndex` (mod (+ (`self.NextPlayerIndex`) 1) (`KismetArrayLibrary.Array_Length` (`self.Players`))))))

(fn `PossessPlayer`
  (params (NewIndex :type Integer))
  (if (`KismetArrayLibrary.Array_IsValidIndex` (`self.Players`) NewIndex)
    (`self.UnPossess`)
    (`self.Possess` (`|GetArrayItem` (`self.Players`) NewIndex))))

(fn `UserConstructionScript`)